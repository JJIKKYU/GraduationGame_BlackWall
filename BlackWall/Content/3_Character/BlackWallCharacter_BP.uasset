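; BlackWallCharacter_BP is a character Blueprint that adds footstep audio and direct input bindings for weapon and combo state.
; FootstepEvent plays the Footsteps sound.
; T or left shoulder equips the weapon and resets the combo count, R unequips, and right shoulder only resets the combo.
; N shows pickup locations, grants MP and resets the combo, using functions defined outside this file.
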(event `FootstepEvent`
  (`AudioComponent.Play` (`self.Footsteps`) 0.0))

(event `Key|N`
  (params (Key :type "Key Structure"))
  (:`Pressed`
    (`self.ShowPickupLocations`)
    (`self.IncrementMP` 100.0)
    (set `self.ComboCnt` 0 :!label _label)))

(event `Key|T`
  (params (Key :type "Key Structure"))
  (:`Pressed`
    (set `self.bWeaponEquipped` true :!label _label_2)
    (goto _label)))

(event `Key|R`
  (params (Key :type "Key Structure"))
  (:`Pressed`
    (set `self.bWeaponEquipped` false)))

(event `Key|Gamepad_RightShoulder`
  (params (Key :type "Key Structure"))
  (:`Pressed`
    (goto _label)))

(event `Key|Gamepad_LeftShoulder`
  (params (Key :type "Key Structure"))
  (:`Pressed`
    (goto _label_2)))

(fn `UserConstructionScript`)